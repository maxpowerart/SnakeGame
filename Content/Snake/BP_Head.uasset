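; Snake game head actor that moves in steps, grows a trail of BP_Segment actors and detects game over.
; Tick, paced by the Movespeed interval plus a Delay, steps the head and shifts segments back-to-front into their predecessors' positions.
; AddSegment spawns tail segments and shortens the tick interval down to a limit.
; Self-overlap or leaving the field shows the end-game UI and pauses the game.
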(event EventBeginPlay
  (bind _defaultsceneroot (Variables|Default|GetDefaultSceneRoot))
  (bind _returnvalue (Transformation|GetWorldLocation _defaultsceneroot))
  (bind (_x _y _z) (Math|Vector|BreakVector _returnvalue))
  ;[1 1 1] Move Z-axis to 0
  (Transformation|SetWorldLocation (Variables|Default|GetDefaultSceneRoot) (Math|Vector|MakeVector _x _y (+ _z -5e+01)) false false)
  (Actor|Tick|SetActorTickInterval (Variables|Default|Getmovespeed)))

(event EventTick
  (params (DeltaSeconds :type Float%20%28single-precision%29))
  (bind _returnvalue (Game|GetPlayerController 0))
  ;[1 1 1] Moving
  (Utilities|FlowControl|Delay 0.2)
  (CallFunction|Move)
  (CallFunction|CheckEndGame)
  (if (Variables|Default|GetisDead)
    (bind _returnvalue_2 (UserInterface|CreateWidget "/Game/UI/WBP_EndGameUI.WBP_EndGameUI_C" (Game|GetPlayerController 0)))
    (UserInterface|Viewport|AddtoViewport _returnvalue_2 0)
    (Variables|Default|SetX_step 0.0)
    (Variables|Default|SetY_step 0.0)
    (Input|DisableInput (Game|Player|GetPlayerPawn 0) _returnvalue)
    (Variables|/Script/Engine.PlayerController|SetbShowMouseCursor _returnvalue true)
    (Input|SetInputModeGameandUI _returnvalue _returnvalue_2 "DoNotLock" false)
    (Game|SetGamePaused true)))

(fn ConstructionScript)

(fn AddSegment
  (bind _segments (Variables|Default|GetSegments))
  (if (== (Utilities|Array|LastIndex (Variables|Default|GetSegments)) -1)
    ;[1 1 1] 1st segment
    (bind _returnvalue (Game|SpawnActorfromClass "/Game/Snake/BP_Segment.BP_Segment_C" (Math|Transform|MakeTransform (Transformation|GetWorldLocation (Variables|Default|GetDefaultSceneRoot)) "0, 0, 0" "1,1,1") "Undefined" 0 0))
    (Utilities|Array|Add (Variables|Default|GetSegments) _returnvalue)
    (else
      ;[1 1 1] Another segments
      (bind _returnvalue_2 (Game|SpawnActorfromClass "/Game/Snake/BP_Segment.BP_Segment_C" (Math|Transform|MakeTransform (Transformation|GetWorldLocation (Variables|/Game/Snake/BP_Segment.BP_Segment_C|GetDefaultSceneRoot (Utilities|Array|Get(acopy) _segments (Utilities|Array|LastIndex _segments)))) "0, 0, 0" "1,1,1") "Undefined" 0 0))
      (Utilities|Array|Add (Variables|Default|GetSegments) _returnvalue_2)))
  (if (> (Variables|Default|Getmovespeed) 0.15)
    (bind _output_get (Variables|Default|Setmovespeed (- (Variables|Default|Getmovespeed) 0.01)))
    (Actor|Tick|SetActorTickInterval _output_get)))

(fn Move
  (bind _defaultsceneroot (Variables|Default|GetDefaultSceneRoot))
  (bind _defaultsceneroot_2 (Variables|Default|GetDefaultSceneRoot))
  (bind _returnvalue (Transformation|GetWorldLocation _defaultsceneroot))
  (bind _returnvalue_2 (Transformation|GetWorldLocation _defaultsceneroot_2))
  (bind (_x _y _z) (Math|Vector|BreakVector _returnvalue_2))
  ;[1 1 1] Move Head
  (Transformation|SetActorLocation (Math|Vector|MakeVector (+ (Variables|Default|Getx_step) _x) (+ _y (Variables|Default|Gety_step)) _z) false true)
  (bind (_arrayindex _arrayelement) (Utilities|Array|ReverseforEachLoop (Variables|Default|GetSegments))
    (:LoopBody
      (if (!= _arrayindex 0)
        ;[1 1 1] Move segments (from end)
        (Transformation|SetWorldLocation (Variables|/Game/Snake/BP_Segment.BP_Segment_C|GetDefaultSceneRoot _arrayelement) (Transformation|GetWorldLocation (Variables|/Game/Snake/BP_Segment.BP_Segment_C|GetDefaultSceneRoot (Utilities|Array|Get(acopy) (Variables|Default|GetSegments) (+ _arrayindex -1)))) false true)
        (else
          ;[1 1 1] Move 1st segment
          (Transformation|SetWorldLocation (Variables|/Game/Snake/BP_Segment.BP_Segment_C|GetDefaultSceneRoot _arrayelement) (Math|Vector|MakeVector (- (.x _returnvalue) (Variables|Default|GetX_step)) (- (.y _returnvalue) (Variables|Default|GetY_step)) (.z _returnvalue)) false true))))))

(fn CheckEndGame
  (bind _defaultsceneroot (Variables|Default|GetDefaultSceneRoot))
  (bind _returnvalue (Transformation|GetWorldLocation _defaultsceneroot))
  (for _array_element (Variables|Default|GetSegments)
    (if (Class|KismetMathLibrary|EqualExactlyVectorVector (Transformation|GetWorldLocation (Variables|Default|GetDefaultSceneRoot)) (Transformation|GetWorldLocation (Variables|/Game/Snake/BP_Segment.BP_Segment_C|GetDefaultSceneRoot _array_element))) ; If snake has self-intersection
      (Variables|Default|SetisDead true)
      (return)))
  (if (Math|Boolean|ORBoolean (> (.x _returnvalue) 4.5e+02) (< (.x _returnvalue) -4.5e+02) (> (.y _returnvalue) 4.5e+02) (< (.y _returnvalue) -4.5e+02)) ; If snake is out of field
    (Variables|Default|SetisDead true)
    (return)
    (else
      (return))))