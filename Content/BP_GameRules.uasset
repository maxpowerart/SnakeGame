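; BP_GameRules holds the rules for a Snake-style game, tracking score, free grid cells and the win condition.
; It fills AwailableCells with a 10x10 grid of world positions, removing the head's cell and, on Update, segment cells.
; Apple pickup increments Score, grows BP_Head and runs Update, though SpawnApple's random cell pick is unwired.
; Tick checks for Score 99, then shows the end-game widget, stops the head and pauses.
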(event Custom|onPIckup
  ;[1 1 1] Collision with apple
  (Math|Integer|IncrementInt (Variables|Default|GetScore)
    (:%20%20
      (bind _asbp_head (Utilities|Casting|CastToBP_Head (Game|Player|GetPlayerPawn 0)))
      (Default|AddSegment _asbp_head)
      (CallFunction|Update))))

(event Custom|Update
  ;[1 1 1] Update free coordinates for apple
  (Utilities|GetAllCells)
  (bind _outactors (Actor|GetAllActorsOfClass "/Game/Snake/BP_Segment.BP_Segment_C"))
  (for _array_element _outactors
    (Utilities|Array|RemoveItem (Variables|Default|GetAwailableCells) (Transformation|GetWorldLocation (Variables|/Game/Snake/BP_Segment.BP_Segment_C|GetDefaultSceneRoot _array_element))))
  (Utilities|RemoveHeadPosition))

(event EventBeginPlay
  ;[1 1 1] Init array of free coordinates
  (Utilities|GetAllCells)
  (Utilities|RemoveHeadPosition))

(event EventTick
  (params (DeltaSeconds :type Float%20%28single-precision%29))
  (bind _returnvalue (Game|GetPlayerController 0))
  ;[1 1 1] Win condition
  (if (== (Variables|Default|GetScore) 99)
    (bind _returnvalue_2 (UserInterface|CreateWidget "/Game/UI/WBP_EndGameUI.WBP_EndGameUI_C" (Game|GetPlayerController 0)))
    (Appearance|SetBrushfromTexture (Variables|/Game/UI/WBP_EndGameUI.WBP_EndGameUI_C|GetImage_48 _returnvalue_2) "/Game/UI/6.6" false)
    (UserInterface|Viewport|AddtoViewport _returnvalue_2 0)
    (bind _asbp_head (Utilities|Casting|CastToBP_Head (Game|Player|GetPlayerPawn 0)))
    (Variables|/Game/Snake/BP_Head.BP_Head_C|SetX_step _asbp_head 0.0)
    (Variables|/Game/Snake/BP_Head.BP_Head_C|SetY_step _asbp_head 0.0)
    (Input|DisableInput (Game|Player|GetPlayerPawn 0) _returnvalue)
    (Variables|/Script/Engine.PlayerController|SetbShowMouseCursor _returnvalue true)
    (Input|SetInputModeGameandUI _returnvalue _returnvalue_2 "DoNotLock" false)
    (Game|SetGamePaused true)))

(fn ConstructionScript)

(fn SpawnApple
  (Actor|GetAllActorsOfClass 0))