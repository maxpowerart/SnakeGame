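; Player controller for a snake-style game that turns directional input into the movement step of the BP_Head pawn.
; Up, Down, Left and Right presses each set XStep and YStep on the head to one grid cell along X or Y.
; When segments exist, it compares the head's position to the first segment's and ignores any turn that would reverse straight back into the body.
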(event EventTick
  (params (DeltaSeconds :type Float%20%28single-precision%29)))

(event Input|ActionEvents|InputActionDown
  (params (Key :type Key%20Structure :default "None"))
  ;[1 1 1] Down
  (:Pressed
    (bind _asbp_head (Utilities|Casting|CastToBP_Head (Game|Player|GetPlayerPawn 0)))
    (if (== (Utilities|Array|Length (Variables|/Game/Snake/BP_Head.BP_Head_C|GetSegments _asbp_head)) 0)
      (Variables|/Game/Snake/BP_Head.BP_Head_C|SetX_step _asbp_head -1e+02 :!label _label)
      (Variables|/Game/Snake/BP_Head.BP_Head_C|SetY_step _asbp_head 0.0)
      (elif (!= (- (.x (Transformation|GetWorldLocation (Variables|/Game/Snake/BP_Head.BP_Head_C|GetDefaultSceneRoot _asbp_head))) (.x (Transformation|GetWorldLocation (Variables|/Game/Snake/BP_Segment.BP_Segment_C|GetDefaultSceneRoot (Utilities|Array|Get(acopy) (Variables|/Game/Snake/BP_Head.BP_Head_C|GetSegments _asbp_head)))))) 1e+02)
        (goto _label)))))

(event Input|ActionEvents|InputActionLeft
  (params (Key :type Key%20Structure :default "None"))
  ;[1 1 1] Left
  (:Pressed
    (bind _asbp_head (Utilities|Casting|CastToBP_Head (Game|Player|GetPlayerPawn 0)))
    (if (== (Utilities|Array|Length (Variables|/Game/Snake/BP_Head.BP_Head_C|GetSegments _asbp_head)) 0)
      (Variables|/Game/Snake/BP_Head.BP_Head_C|SetX_step _asbp_head 0.0 :!label _label)
      (Variables|/Game/Snake/BP_Head.BP_Head_C|SetY_step _asbp_head -1e+02)
      (elif (!= (- (.y (Transformation|GetWorldLocation (Variables|/Game/Snake/BP_Head.BP_Head_C|GetDefaultSceneRoot _asbp_head))) (.y (Transformation|GetWorldLocation (Variables|/Game/Snake/BP_Segment.BP_Segment_C|GetDefaultSceneRoot (Utilities|Array|Get(acopy) (Variables|/Game/Snake/BP_Head.BP_Head_C|GetSegments _asbp_head)))))) 1e+02)
        (goto _label)))))

(event Input|ActionEvents|InputActionUp
  (params (Key :type Key%20Structure :default "None"))
  ;[1 1 1] Up
  (:Pressed
    (bind _asbp_head (Utilities|Casting|CastToBP_Head (Game|Player|GetPlayerPawn 0)))
    (if (== (Utilities|Array|Length (Variables|/Game/Snake/BP_Head.BP_Head_C|GetSegments _asbp_head)) 0)
      (Variables|/Game/Snake/BP_Head.BP_Head_C|SetX_step _asbp_head 1e+02 :!label _label)
      (Variables|/Game/Snake/BP_Head.BP_Head_C|SetY_step _asbp_head 0.0)
      (elif (!= (- (.x (Transformation|GetWorldLocation (Variables|/Game/Snake/BP_Head.BP_Head_C|GetDefaultSceneRoot _asbp_head))) (.x (Transformation|GetWorldLocation (Variables|/Game/Snake/BP_Segment.BP_Segment_C|GetDefaultSceneRoot (Utilities|Array|Get(acopy) (Variables|/Game/Snake/BP_Head.BP_Head_C|GetSegments _asbp_head)))))) -1e+02)
        (goto _label)))))

(event Input|ActionEvents|InputActionRight
  (params (Key :type Key%20Structure :default "None"))
  ;[1 1 1] Right
  (:Pressed
    (bind _asbp_head (Utilities|Casting|CastToBP_Head (Game|Player|GetPlayerPawn 0)))
    (if (== (Utilities|Array|Length (Variables|/Game/Snake/BP_Head.BP_Head_C|GetSegments _asbp_head)) 0)
      (Variables|/Game/Snake/BP_Head.BP_Head_C|SetX_step _asbp_head 0.0 :!label _label)
      (Variables|/Game/Snake/BP_Head.BP_Head_C|SetY_step _asbp_head 1e+02)
      (elif (!= (- (.y (Transformation|GetWorldLocation (Variables|/Game/Snake/BP_Head.BP_Head_C|GetDefaultSceneRoot _asbp_head))) (.y (Transformation|GetWorldLocation (Variables|/Game/Snake/BP_Segment.BP_Segment_C|GetDefaultSceneRoot (Utilities|Array|Get(acopy) (Variables|/Game/Snake/BP_Head.BP_Head_C|GetSegments _asbp_head)))))) -1e+02)
        (goto _label)))))

(fn ConstructionScript)